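; Player character Blueprint with yaw-relative movement, mouse-wheel camera zoom and projectile shooting from a muzzle socket.
; Shooting picks a power or normal projectile from the ammo component's improved state and count, with DoOnce plus Delay as per-type cooldowns.
; Enemy capsule overlaps damage the health component.
; Its death event, marked unfinished, prints a message, pauses, then calls a game mode restart after a delay.
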(event OnComponentBeginOverlap(CapsuleComponent)
  (params (OverlappedComponent :type Primitive%20Component%20Object%20Reference) (OtherActor :type Actor%20Object%20Reference) (OtherComp :type Primitive%20Component%20Object%20Reference) (OtherBodyIndex :type Integer) (bFromSweep :type Boolean) (SweepResult :type Hit%20Result%20Structure%20%28by%20ref%29))
  ;[1 1 1] Getting Damage on overlaps with Enemy
  (Utilities|Casting|CastToBP_Enemy OtherActor)
  (Default|GetDamage (Variables|Default|GetBPC_Health) (Variables|PlayerProperties|GetEnemyDamage)))

(event EDDeath(BPC_Health)
  ;[1 1 1] Death mechanics (unfinished)
  (bind _astop_down_game_mode (Utilities|Casting|CastToTopDownGameMode (Game|GetGameMode)))
  (Development|PrintString "Вы погибли!")
  (Game|SetGamePaused true)
  (Utilities|FlowControl|Delay 3.0)
  (Class|GameMode|RestartGame _astop_down_game_mode))

(event Custom|Shot
  ;[1 1 1] Spawning projectile
  (bind _bp_projectile (Variables|Spawns|GetBP_Projectile)
    (:then
      (Game|SpawnActorfromClass _bp_projectile (Transformation|GetSocketTransform (Variables|Character|GetMesh) "MuzzleSocket" "RTS_World") "Undefined" 0 0))
    (:else)))

(event Custom|PowerShot
  ;[1 1 1] Spawning power projectile
  (bind _bp_powerprojectile (Variables|Spawns|GetBP_PowerProjectile)
    (:then
      (Game|SpawnActorfromClass _bp_powerprojectile (Transformation|GetSocketTransform (Variables|Character|GetMesh) "MuzzleSocket" "RTS_World") "Undefined" 0 0))
    (:else)))

(event EventTick
  (params (DeltaSeconds :type Float%20%28single-precision%29))
  ;[1 1 1] UI debug
)

(event Input|ActionEvents|InputActionShoot
  (params (Key :type Key%20Structure :default "None"))
  (bind _bpc_ammo (Variables|Default|GetBPC_Ammo))
  ;[1 1 1] Shooting
  (:Pressed
    (Utilities|ShootingMechanics (Variables|/Game/Blueprints/Components/BPC_Ammo.BPC_Ammo_C|GetShot%20Improved _bpc_ammo) (Variables|/Game/Blueprints/Components/BPC_Ammo.BPC_Ammo_C|GetPower%20Shot%20Ammo _bpc_ammo))))

(event Input|AxisEvents|InputAxisMoveForwardBack
  (params (AxisValue :type Float%20%28single-precision%29))
  ;[1 1 1] Player control
  (Pawn|Input|AddMovementInput (Math|Vector|GetForwardVector (Math|Rotator|MakeRotator 0.0 0.0 (.yaw (Pawn|GetControlRotation :!class /Script/Engine.Pawn)))) AxisValue false))

(event Input|AxisEvents|InputAxisMoveLeftRight
  (params (AxisValue :type Float%20%28single-precision%29))
  ;[1 1 1] Player control
  (Pawn|Input|AddMovementInput (Math|Vector|GetRightVector (Math|Rotator|MakeRotator 0.0 0.0 (.yaw (Pawn|GetControlRotation :!class /Script/Engine.Pawn)))) AxisValue false))

(event Input|AxisEvents|InputAxisLookLeftRight
  (params (AxisValue :type Float%20%28single-precision%29))
  ;[1 1 1] Camera control
  (Pawn|Input|AddControllerYawInput AxisValue))

(event Input|MouseEvents|MouseWheelUp
  (params (Key :type Key%20Structure :default "None"))
  (bind _springarm (Variables|Default|GetSpringArm))
  ;[1 1 1] Camera control
  (:Pressed
    (if (>= (Variables|/Script/Engine.SpringArmComponent|GetTargetArmLength _springarm) 3e+02)
      (Variables|/Script/Engine.SpringArmComponent|SetTargetArmLength _springarm (- (Variables|/Script/Engine.SpringArmComponent|GetTargetArmLength _springarm) 5e+01)))))

(event Input|MouseEvents|MouseWheelDown
  (params (Key :type Key%20Structure :default "None"))
  (bind _springarm (Variables|Default|GetSpringArm))
  ;[1 1 1] Camera control
  (:Pressed
    (if (<= (Variables|/Script/Engine.SpringArmComponent|GetTargetArmLength _springarm) 2e+03)
      (Variables|/Script/Engine.SpringArmComponent|SetTargetArmLength _springarm (+ (Variables|/Script/Engine.SpringArmComponent|GetTargetArmLength _springarm) 5e+01)))))

(fn ConstructionScript
  (|CallParentFunction))