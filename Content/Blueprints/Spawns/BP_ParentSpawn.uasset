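; BP_ParentSpawn is a universal spawner that periodically places random pickups or enemies in the level.
; A looping timer picks a random SpawnClass entry, with separate rolls for the validity check and the spawn.
; GetSpawnLocation samples a point in a scale-derived box around the first TriggerBox found.
; IsNotSavePoint forces a re-roll while that point lies inside a box sized by the player's SafeArea capsule radius.
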(event Custom|SpawnActor
  (bind _spawnclass (Variables|SpawnProperties|GetSpawnClass))
  (bind _maxspawnrange (Variables|SpawnProperties|GetMaxSpawnRange))
  (bind _returnvalue (Math|Random|RandomIntegerinRange 0 _maxspawnrange))
  (bind _output (Utilities|Array|Get(acopy) _spawnclass _returnvalue))
  ;[1 1 1] Universal spawner for Pickups and Enemies
  (if (Utilities|IsValidClass _output)
    (bind _spawnlocation (CallFunction|GetSpawnLocation :!label _label))
    (bind _output_get (Variables|Default|SetSpawnLocation _spawnlocation))
    (if (CallFunction|IsNotSavePoint _output_get)
      (goto _label)
      (else
        (Game|SpawnActorfromClass _output (Math|Transform|MakeTransform (Variables|Default|GetSpawnLocation) "0, 0, 0" "1,1,1") "AdjustIfPossibleButDontSpawnIfColliding" 0 0)))
    (else
      (Development|PrintString "Invalid Spawn Class!" true true "(R=0.000000,G=0.660000,B=1.000000,A=1.000000)" 0.0))))

(event EventBeginPlay
  ;[1 1 1] Universal spawner for Pickups and Enemies
  (Utilities|Time|SetTimerbyEvent (delegate Custom|SpawnActor) (Variables|SpawnProperties|GetSpawnDelay) true))

(fn ConstructionScript)

(fn GetSpawnLocation
  ;[1 1 1] Getting a random spawn point
  (bind _outactors (Actor|GetAllActorsOfClass "/Script/Engine.TriggerBox"))
  (return (Math|Random|RandomPointinBoundingBox (.location (Transformation|GetActorTransform (Utilities|Array|Get(acopy) _outactors))) (* "40.000000,40.000000,40.000000" (.scale (Transformation|GetActorTransform (Utilities|Array|Get(acopy) _outactors)))))))

(fn IsNotSavePoint
  (params (SpawnLocation :type Vector))
  ;[1 1 1] Spawn point is not to be close then 2 meters from Player
  (bind _asbp_player (Utilities|Casting|CastToBP_Player (Game|GetPlayerCharacter 0)))
  (return (Math|Geometry|IsPointinBox SpawnLocation (Transformation|GetActorLocation _asbp_player) (Math|Conversions|ToVector(Float) (Components|Capsule|GetScaledCapsuleRadius (Variables|/Game/Blueprints/Characters/BP_Player.BP_Player_C|GetSafe%20area _asbp_player))))))