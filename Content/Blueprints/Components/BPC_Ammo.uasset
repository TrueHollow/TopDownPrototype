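; BPC_Ammo is a component that tracks power shot ammo for its owner.
; AddPowerAmmo raises the count and sets ShotImproved, while WastePowerAmmo lowers it without clamping or clearing that flag.
; Both functions write a formatted "Power shot" count into the second AmmoType entry, then fire the AmmoChanged dispatcher to notify listeners.
; It has no active event logic and changes only through these calls.
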(event EventBeginPlay)

(event EventTick
  (params (DeltaSeconds :type Float%20%28single-precision%29)))

(fn AddPowerAmmo
  (params (AmmoValue :type Integer))
  (Variables|Default|SetShot%20Improved true)
  (bind _output_get (Variables|Default|SetPower%20Shot%20Ammo (+ (Variables|Default|GetPower%20Shot%20Ammo) AmmoValue)))
  (|SetBy-RefVar (Utilities|Array|Get(acopy) (Variables|Default|GetAmmo%20Type) 1) (Utilities|Text|FormatText "Power shot: {Ammo}" _output_get))
  (Default|CallEDAmmoChanged))

(fn WastePowerAmmo
  (params (WasteValue :type Integer))
  (bind _output_get (Variables|Default|SetPower%20Shot%20Ammo (- (Variables|Default|GetPower%20Shot%20Ammo) WasteValue)))
  (|SetBy-RefVar (Utilities|Array|Get(acopy) (Variables|Default|GetAmmo%20Type) 1) (Utilities|Text|FormatText "Power shot: {Ammo}" _output_get))
  (Default|CallEDAmmoChanged))