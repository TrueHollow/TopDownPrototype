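; BPC_Health is a health component that tracks Health against MaxHealth and handles damage, healing and death.
; GetDamage subtracts damage, floors Health at zero and fires the death dispatcher via IsDead, including on hits when already dead.
; RestoreHealth caps healing at MaxHealth; both functions broadcast the health-changed dispatcher before clamping.
; RestoreMaxHealth refills Health without broadcasting, and the component does not tick.
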(event EventBeginPlay)

(event EventTick
  (params (DeltaSeconds :type Float%20%28single-precision%29)))

(fn GetDamage
  (params (Damage :type Float%20%28single-precision%29))
  (bind _dead (CallFunction|IsDead))
  (if _dead
    (Default|CallEDDeath)
    (else
      (bind _output_get (Variables|HealthComponent|SetHealth (- (Variables|HealthComponent|GetHealth) Damage)))
      (Default|CallEDHealthChanged)
      (if (< _output_get 0.0)
        (Variables|HealthComponent|SetHealth 0.0))
      (bind _dead_2 (CallFunction|IsDead))
      (if _dead_2
        (Default|CallEDDeath)
        (else
          (return (Variables|HealthComponent|GetHealth)))))))

(fn RestoreHealth
  (params (HealValue :type Float%20%28single-precision%29))
  (if (< (Variables|HealthComponent|GetHealth) (Variables|HealthComponent|GetMaxHealth))
    (bind _output_get (Variables|HealthComponent|SetHealth (+ (Variables|HealthComponent|GetHealth) HealValue)))
    (Default|CallEDHealthChanged)
    (if (> _output_get (Variables|HealthComponent|GetMaxHealth))
      (Variables|HealthComponent|SetHealth (Variables|HealthComponent|GetMaxHealth)))
    (return (Variables|HealthComponent|GetHealth))))

(fn RestoreMaxHealth
  (bind _output_get (Variables|HealthComponent|SetHealth (Variables|HealthComponent|GetMaxHealth)))
  (return _output_get))

(fn IsDead
  (return (<= (Variables|HealthComponent|GetHealth) 0.0)))